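; Interactable candle that reveals hidden 3D text when powder is used on it.
; Each interaction alternates the point light on and off through a FlipFlop, with a timeline animating intensity on light-up and stopping at zero on switch-off.
; Using powder recolors the light to the powder color and makes the text visible, regardless of whether the candle is lit.
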(event Custom|UpLight
  (bind _change_intensity (Timeline|Timeline PlayFromStart)
    (:Update
      (bind _output_get (Variables|Default|SetIntensity (Math|Float|Lerp 0.0 8e+03 _change_intensity)))
      (Rendering|Components|Light|SetIntensity (Variables|Default|GetPointLight) _output_get))))

(event Custom|OffLight
  (Rendering|Components|Light|SetIntensity (Variables|Default|GetPointLight) 0.0)
  (bind _change_intensity (Timeline|Timeline Stop)
    (:Update
      (bind _output_get (Variables|Default|SetIntensity (Math|Float|Lerp 0.0 8e+03 _change_intensity)))
      (Rendering|Components|Light|SetIntensity (Variables|Default|GetPointLight) _output_get))))

(event EventInetract
  (Utilities|FlowControl|FlipFlop
    (:A
      (CallFunction|UpLight))
    (:B
      (CallFunction|OffLight))))

(event EventUsePowder
  (Rendering|Components|Light|SetLightColor (Variables|Default|GetPointLight) (Variables|Default|GetPowder%20Color) true)
  (Rendering|SetVisibility (Variables|Default|GetText3D) true false))

(fn ConstructionScript)